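; BP_CaveFlyer is a player-controlled flyer that handles basic movement input and nothing else.
; Forward and back action presses add movement along the control rotation's full forward vector, pitch included.
; Left and right presses use the right vector of a zero rotation, so they follow a fixed world axis.
; Movement fires only on press, and Turn and LookUp feed constant zero to yaw and pitch, leaving look input inert.
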(event `InputAction|MoveForward`
  (params (Key :type "Key Structure"))
  (:`Pressed`
    (`self.AddMovementInput` (`KismetMathLibrary.GetForwardVector` (`self.GetControlRotation`)))))

(event `InputAxis|Turn`
  (params (AxisValue :type "Float (single-precision)"))
  (`self.AddControllerYawInput` 0.0))

(event `InputAction|MoveBack`
  (params (Key :type "Key Structure"))
  (:`Pressed`
    (`self.AddMovementInput` (`KismetMathLibrary.GetForwardVector` (`self.GetControlRotation`)) -1.0)))

(event `InputAxis|LookUp`
  (params (AxisValue :type "Float (single-precision)"))
  (`self.AddControllerPitchInput` 0.0))

(event `InputAction|MoveRight`
  (params (Key :type "Key Structure"))
  (:`Pressed`
    (`self.AddMovementInput` (`KismetMathLibrary.GetRightVector` (struct)))))

(event `InputAction|MoveLeft`
  (params (Key :type "Key Structure"))
  (:`Pressed`
    (`self.AddMovementInput` (`KismetMathLibrary.GetRightVector` (struct)) -1.0)))

(fn `UserConstructionScript`)